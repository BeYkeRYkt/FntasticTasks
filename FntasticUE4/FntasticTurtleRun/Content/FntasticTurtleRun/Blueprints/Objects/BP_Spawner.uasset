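; BP_Spawner is a placeable spawner that, when activated, spawns a configurable AI entity with its controller, behavior tree, sounds and name passed in.
; Activation plays a sound and particle effect at the spawner's mesh, then spawns the entity at the spawner's location and rotation.
; It then writes the start position and the DestinationPoint actor's location into the entity's BP_AIController blackboard as start and target positions.
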(event `/Game/FntasticTurtleRun/Blueprints/Interaction/BPI_Interaction.OnActivate`
  (bind _returnvalue (`SceneComponent.K2_GetComponentLocation` (`self.SM_MERGED_SM_Box_2`)))
  ;[1 1 1] get forward spawn position
  (set `self.StartPosition` (+ (`self.K2_GetActorLocation`) (* (`KismetMathLibrary.GetForwardVector` (`self.K2_GetActorRotation`)) 0.0)))
  ;[1 1 1] get target position
  (set `self.TargetPosition` (`self.K2_GetActorLocation` (`self.DestinationPoint`)))
  ;[1 1 1] Spawn effects
  (`GameplayStatics.SpawnSoundAtLocation` "/Game/ThirdParty/HalfLife2/Sounds/Gates/default_move.default_move" _returnvalue (struct) 1.0 1.0 0.0 "/Game/FntasticTurtleRun/Blueprints/Sounds/DefaultSoundAttenuation.DefaultSoundAttenuation" null)
  (`GameplayStatics.SpawnEmitterAtLocation` (`self.SpawnEffect`) _returnvalue (struct) (1.0 1.0 1.0) true "AutoRelease")
  (bind _returnvalue_2 (`|SpawnActorFromClass` (`self.SpawnEntity`) (`KismetMathLibrary.MakeTransform` (`self.StartPosition`) (`SceneComponent.K2_GetComponentRotation` (`self.DefaultSceneRoot`))) "AlwaysSpawn" "OverrideRootScale" null (`self.AIController`) (`self.AttachSound`) (`self.DeathSound`) (`self.LastWordsSound`) (`self.BehaviorTree`) (`self.Entity name`) null))
  ;[1 1 1] Setup AI params
  (bind _asbp_aicontroller (cast `/Game/FntasticTurtleRun/Blueprints/AI/Controllers/BP_AIController` (`AIBlueprintHelperLibrary.GetAIController` _returnvalue_2)))
  (`/Game/FntasticTurtleRun/Blueprints/AI/Controllers/BP_AIController.UpdateBlackboardVector` _asbp_aicontroller (`self.StartPositionKey`) (`self.StartPosition`))
  (`/Game/FntasticTurtleRun/Blueprints/AI/Controllers/BP_AIController.UpdateBlackboardVector` _asbp_aicontroller (`self.TargetPositionKey`) (`self.TargetPosition`)))

(fn `UserConstructionScript`)