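; BP_Turtle is the turtle character for FntasticTurtleRun, extending a parent entity class with effects and sounds.
; An attached emitter marks the turtle while an AI is attached to it and is destroyed on detach.
; Interaction kills the turtle, and death spawns a randomly scaled explosion with sound before the parent handling runs.
; Tick uses a DoOnce to start a looping footstep timer during grounded movement and clears it otherwise.
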(event `self.OnEntityAttachedByAI`
  (params (Notify :type Boolean))
  ;[1 1 1] OnEntityAttachedByAI
  (`parent.OnEntityAttachedByAI` Notify)
  (bind _returnvalue (`GameplayStatics.SpawnEmitterAttached` (`self.AttachedAIEffect`) (`self.CustomMesh`) "None" (0.0 0.0 0.0) (struct) (1.0 1.0 1.0) "KeepRelativeOffset" true "AutoRelease"))
  (set `self.ParticleComponent` _returnvalue))

(event `self.OnEntityUnattachedByAI`
  (bind _particlecomponent (`self.ParticleComponent`))
  ;[1 1 1] OnEntityUnattachedByAI
  (`parent.OnEntityUnattachedByAI`)
  (`/Engine/EditorBlueprintResources/StandardMacros.IsValid` _particlecomponent
    (:`Is Valid`
      (`ActorComponent.K2_DestroyComponent` _particlecomponent))))

(event `self.ReceiveBeginPlay`
  (`parent.ReceiveBeginPlay`))

(event `self.OnEntityDeath`
  ;[1 1 1] OnEntityDeath
  (`GameplayStatics.SpawnEmitterAtLocation` "/Game/FXVarietyPack/Particles/P_ky_explosion.P_ky_explosion" (`self.K2_GetActorLocation`) (struct) (* (`KismetMathLibrary.RandomUnitVector`) (`self.sizeScale`)) true "AutoRelease")
  (`self.playSound` "/Game/ThirdParty/TeamFortess2/Sounds/Weapons/ExplodeSound.ExplodeSound" false "/Game/FntasticTurtleRun/Blueprints/Sounds/DefaultSoundAttenuation.DefaultSoundAttenuation")
  (`parent.OnEntityDeath`))

(event `/Game/FntasticTurtleRun/Blueprints/Interaction/BPI_Interaction.OnInteraction`
  (params (From :type "Character Object Reference"))
  ;[1 1 1] Interaction
  (`self.killEntity`))

(event `OnEntityWalking`
  ;[1 1 1] Footsteps
  (`self.playSound` "/Game/ThirdParty/generic_footsteps/sound/player/footsteps/FootstepsWood_Sounds.FootstepsWood_Sounds" false "/Game/FntasticTurtleRun/Blueprints/Sounds/DefaultSoundAttenuation.DefaultSoundAttenuation" 0.25))

(event `self.ReceiveTick`
  (params (DeltaSeconds :type "Float (single-precision)"))
  ;[1 1 1] Footsteps
  (`parent.ReceiveTick` DeltaSeconds)
  (if (and (!= (`self.GetVelocity`) (0.0 0.0 0.0)) (`NavMovementComponent.IsMovingOnGround` (`self.CharacterMovement`)))
    (`/Engine/EditorBlueprintResources/StandardMacros.DoOnce` false :!label _label
      (:`Completed`
        (bind _returnvalue (`KismetSystemLibrary.K2_SetTimerDelegate` (delegate `OnEntityWalking`) 0.25 true))))
    (else
      (`KismetSystemLibrary.K2_ClearAndInvalidateTimerHandle` _returnvalue)
      (goto _label :!via `Reset`))))

(fn `UserConstructionScript`
  (`parent.UserConstructionScript`))