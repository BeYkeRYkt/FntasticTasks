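; BP_Entity is a base AI character for TurtleRun that spawns, attaches, and dies with sound feedback and shows a name label.
; Spawning runs its behavior tree on BP_AIController, and attach and death events play sounds attached to the mesh.
; Killing stops the tree and destroys the actor; a delayed variant first plays trigger and last-words sounds.
; A text render shows the entity name and turns toward the player camera each tick.
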(event `self.OnEntityAttachedByAI`
  (params (Notify :type Boolean))
  ;[1 1 1] On Entity Attached by AI
  (if Notify
    (`self.playSound` (`self.AttachSound`) true)))

(event `self.OnEntitySpawn`
  ;[1 1 1] OnEntitySpawn
  (bind _btaicontroller (`self.GetBTAIController`))
  (`/Game/FntasticTurtleRun/Blueprints/AI/Controllers/BP_AIController.RunBT` _btaicontroller (`self.BehaviorTree`)))

(event `self.OnEntityDeath`
  ;[1 1 1] OnEntityDeath
  (`self.playSound` (`self.DeathSound`)))

(event `self.playSound`
  (params (sound :type "SoundBase Object Reference") (stopWhenDestroyed :type Boolean))
  ;[1 1 1] Play sound
  (`GameplayStatics.SpawnSoundAttached` sound (`self.Mesh`) "None" (0.0 0.0 0.0) (struct) "KeepRelativeOffset" stopWhenDestroyed 1.0 1.0 0.0 "/Game/FntasticTurtleRun/Blueprints/Sounds/DefaultSoundAttenuation.DefaultSoundAttenuation" null))

(event `self.killEntity`
  ;[1 1 1] Kill Entity
  (bind _btaicontroller (`self.GetBTAIController`))
  (`/Game/FntasticTurtleRun/Blueprints/AI/Controllers/BP_AIController.StopBT` _btaicontroller)
  (`self.OnEntityDeath`)
  (`self.K2_DestroyActor`))

(event `self.killEntityWithDelay`
  (params (time :type "Float (single-precision)"))
  ;[1 1 1] Kill Entity with Delay
  (bind _btaicontroller (`self.GetBTAIController`))
  (`/Game/FntasticTurtleRun/Blueprints/AI/Controllers/BP_AIController.StopBT` _btaicontroller)
  (`self.playSound` "/Game/ThirdParty/TeamFortess2/Sounds/Weapons/cart_explode_trigger.cart_explode_trigger")
  (`KismetSystemLibrary.Delay` 0.5)
  (`self.playSound` (`self.LastWordsSound`) true)
  (`KismetSystemLibrary.Delay` time)
  (`self.killEntity`))

(event `self.ReceiveBeginPlay`
  ;[1 1 1] Text
  (`TextRenderComponent.K2_SetText` (`self.TextRender`) (`self.Entity Name`)))

(event `self.ReceiveTick`
  (params (DeltaSeconds :type "Float (single-precision)"))
  (bind _textrender (`self.TextRender`))
  ;[1 1 1] Text rotation
  (`SceneComponent.K2_SetWorldRotation` _textrender (`KismetMathLibrary.FindLookAtRotation` (`SceneComponent.K2_GetComponentLocation` _textrender) (`self.K2_GetActorLocation` (`GameplayStatics.GetPlayerCameraManager` 0))) false false))

(fn `GetBTAIController`
  (returns (BTAIController :type "/Game/FntasticTurtleRun/Blueprints/AI/Controllers/BP_AIController Object Reference"))
  (bind _asbp_aicontroller (cast `/Game/FntasticTurtleRun/Blueprints/AI/Controllers/BP_AIController` (`AIBlueprintHelperLibrary.GetAIController` self)))
  (return _asbp_aicontroller))

(fn `UserConstructionScript`
  (set `self.AIControllerClass` (`self.AI_Controller`)))